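; Level 2 scenario Blueprint that scripts a quest beat in which the player pecks a trinket and Rook the Keeper decides to keep it.
; ActivateScenario makes the trinket peckable; pecking it snaps the gate open, enables the outer trigger and loads Rook's dialogue about it.
; When that conversation finishes, the handler unbinds itself and swaps in a short dismissive line set for any later talk.
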(event Custom|ActivateScenario
  (bind _trinket (Variables|Default|GetTrinket))
  (Default|SetPeckable _trinket true)
  (EventDispatchers|AssignOnPecked _trinket (delegate Custom|TrinketPecked)))

(event Custom|TrinketPecked
  (bind _generalscenario (Variables|Default|GetGeneralScenario))
  (bind _rook (Variables|/Game/Blueprints/LevelScenario.LevelScenario_C|GetRook _generalscenario))
  (Default|SnapGateOpen _generalscenario)
  (Default|EnableOuterTrigger _generalscenario)
  (Variables|/Game/ThirdPerson/Blueprints/CrowCharacter_BP.CrowCharacter_BP_C|SetConversationStruct _rook (Utilities|Struct|MakeConversationStruct (Utilities|Array|MakeArray "What do you have there in your beak?" "Oh it's the trinket! Oh, wow, it's so shiny. Marvelous..." "Hmmm..." "You think she'll mind if I keep it?" "Yeah, you're right, it wouldn't be nice." "But what if she never finds out that we found it? We tell her it's lost." "I understand it's important. It's a family heirloom, a gift from her late husband, yada yada! But she has to learn how to let go." "And I'm going to teach her that lesson." "Anyways, you're free for the night, I've no tasks left.") "Rook the Keeper"))
  (EventDispatchers|AssignConversationFinished _rook (delegate Custom|ConvFinished)))

(event Custom|ConvFinished
  (bind _generalscenario (Variables|Default|GetGeneralScenario))
  (bind _rook (Variables|/Game/Blueprints/LevelScenario.LevelScenario_C|GetRook _generalscenario))
  (EventDispatchers|UnbindEventfromConversationFinished _rook (delegate Custom|ConvFinished))
  (Variables|/Game/ThirdPerson/Blueprints/CrowCharacter_BP.CrowCharacter_BP_C|SetConversationStruct _rook (Utilities|Struct|MakeConversationStruct (Utilities|Array|MakeArray "So shiny..." "I've no more tasks for you! Get lost!") "Rook the Keeper")))

(fn ConstructionScript)