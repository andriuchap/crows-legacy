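; A trigger volume that closes a gate by playing a level sequence when the third-person character overlaps it.
; On overlap it stops a competing sequence if playing, plays its own, then disables itself, optionally showing the mission on the character.
; When the sequence it triggered finishes, it either plays a cinematic impact sound (mission shown) or calls MissionComplete on the level scenario.
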(event OnComponentBeginOverlap(CollisionComponent)
  (params (OverlappedComponent :type Primitive%20Component%20Object%20Reference) (OtherActor :type Actor%20Object%20Reference) (OtherComp :type Primitive%20Component%20Object%20Reference) (OtherBodyIndex :type Integer) (bFromSweep :type Boolean) (SweepResult :type Hit%20Result%20Structure%20%28by%20ref%29))
  (bind _othersequence (Variables|Default|GetOtherSequence))
  (bind _sequenceplayer (Variables|/Script/LevelSequence.LevelSequenceActor|GetSequencePlayer _othersequence))
  (if (Variables|Default|GetEnabled)
    (bind _asbp_third_person_character (Utilities|Casting|CastToBP_ThirdPersonCharacter OtherActor))
    (if (Variables|Default|GetShouldShowMission)
      (Default|ShowMIssion _asbp_third_person_character))
    (if (Audio|Components|Audio|IsPlaying _sequenceplayer)
      (Sequencer|Player|Stop _sequenceplayer :!class /Script/MovieScene.MovieSceneSequencePlayer))
    (Sequencer|Player|Play (Variables|/Script/LevelSequence.LevelSequenceActor|GetSequencePlayer (Variables|Default|GetMySequence)) :!class /Script/MovieScene.MovieSceneSequencePlayer)
    (Variables|Default|SetEnabled false)
    (Variables|Default|SetI%20Triggered%20Gate%20Close true)))

(event Custom|OnFinished_Event
  (if (Variables|Default|GetI%20Triggered%20Gate%20Close)
    (Variables|Default|SetI%20Triggered%20Gate%20Close false)
    (Audio|PlaySound2D "/Game/Audio/CinematicImpact/CinematicImpact.CinematicImpact" 1.0 1.0 0.0 0 0)))

(event Custom|FinishMusic
  (if (Variables|Default|GetI%20Triggered%20Gate%20Close)
    (Variables|Default|SetI%20Triggered%20Gate%20Close false)
    (Default|MissionComplete (Variables|Default|GetLevelScenario))))

(event EventBeginPlay
  (bind _mysequence (Variables|Default|GetMySequence))
  (bind _sequenceplayer (Variables|/Script/LevelSequence.LevelSequenceActor|GetSequencePlayer _mysequence))
  (if (Variables|Default|GetShouldShowMission)
    (EventDispatchers|AssignOnFinished _sequenceplayer (delegate Custom|OnFinished_Event))
    (else
      (EventDispatchers|AssignOnFinished _sequenceplayer (delegate Custom|FinishMusic)))))

(fn ConstructionScript)