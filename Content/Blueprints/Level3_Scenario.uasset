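; Level 3 scenario actor that runs the "Cleanup the graveyard" quest, from mission start to the closing dialogue with Rook the Keeper.
; Activation sets up the gate, trigger, music and gravestones through GeneralScenario, then binds every Peckable to a shared counter.
; The second peck preloads completion flavor text onto remaining items.
; The third reopens the gate and arms Rook's debrief, which switches to a dismissal line once finished.
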(event Custom|ActivateScenario
  (bind _generalscenario (Variables|Default|GetGeneralScenario))
  (bind _asbp_third_person_character (Utilities|Casting|CastToBP_ThirdPersonCharacter (Game|Player|GetPlayerPawn 0)))
  (Default|SetMission _asbp_third_person_character "Cleanup the graveyard.")
  (Default|EnableInnerTrigger _generalscenario)
  (Default|OpenGate _generalscenario)
  (Default|PlayLevelMusic _generalscenario)
  (Default|SetShowSpecified (Variables|/Game/Blueprints/LevelScenario.LevelScenario_C|GetGravestoneController _generalscenario) (Variables|Default|GetNewGravestones))
  (for _array_element (Variables|Default|GetPeckables)
    (Default|SetPeckable _array_element true)
    (EventDispatchers|AssignOnPecked _array_element (delegate Custom|Pecked))))

(event Custom|Pecked
  (bind _generalscenario (Variables|Default|GetGeneralScenario))
  (bind _rook (Variables|/Game/Blueprints/LevelScenario.LevelScenario_C|GetRook _generalscenario))
  (bind _output_get (Variables|Default|SetPeckedItems (+ (Variables|Default|GetPeckedItems) 1)))
  (Utilities|FlowControl|Sequence
    (:then_0
      (if (== _output_get 2)
        (for _array_element (Variables|Default|GetPeckables)
          (Utilities|IsValid _array_element
            (:Is%20Valid
              (Variables|/Game/Blueprints/PeckableActor_BP.PeckableActor_BP_C|SetFlavorText _array_element "The graveyard appears much cleaner now! Return to Rook the Keeper."))))))
    (:then_1
      (if (== _output_get 3)
        (Default|SnapGateOpen _generalscenario)
        (Default|EnableOuterTrigger _generalscenario)
        (Variables|/Game/ThirdPerson/Blueprints/CrowCharacter_BP.CrowCharacter_BP_C|SetConversationStruct _rook (Utilities|Struct|MakeConversationStruct (Utilities|Array|MakeArray "My precious little shiny..." "Oh, you're back! Did you clean up the graveyard?" "Good, goooood. What's that you say?" "New gravestones rose up? That's nonsense! How can that happen if we didn't bury anyone new tonight?" "I don't have time for your crazy stories! We're done for tonight, you can do whatever you want now!") "Rook the Keeper"))
        (EventDispatchers|BindEventtoConversationFinished _rook (delegate Custom|ConversationFinished))))))

(event Custom|ConversationFinished
  (EventDispatchers|UnbindEventfromConversationFinished (Variables|/Game/Blueprints/LevelScenario.LevelScenario_C|GetRook (Variables|Default|GetGeneralScenario)) (delegate Custom|ConversationFinished))
  (Variables|/Game/ThirdPerson/Blueprints/CrowCharacter_BP.CrowCharacter_BP_C|SetConversationStruct (Variables|/Game/Blueprints/LevelScenario.LevelScenario_C|GetRook (Variables|Default|GetGeneralScenario)) (Utilities|Struct|MakeConversationStruct (Utilities|Array|MakeArray "Get away now! I have things to do! Shiny...") "Rook the Keeper")))

(fn ConstructionScript)