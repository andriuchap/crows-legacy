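; Level 1 scenario script that runs the completion of the walnut-pecking first task and hands the game over to Level 2.
; Pecking the walnut snaps the gate open, teleports Rook the Keeper to a target spot with completion dialogue, and enables the outer trigger.
; When that conversation finishes, it sends Rook to wait, sets the trinket mission, enables the inner trigger, opens the gate, starts music and activates Level 2.
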(event Custom|WalnutPecked
  (bind _generalscenario (Variables|Default|GetGeneralScenario))
  (bind _generalscenario_2 (Variables|Default|GetGeneralScenario))
  (bind _rook (Variables|/Game/Blueprints/LevelScenario.LevelScenario_C|GetRook _generalscenario))
  (bind _rook_2 (Variables|/Game/Blueprints/LevelScenario.LevelScenario_C|GetRook _generalscenario_2))
  (Default|SnapGateOpen _generalscenario)
  (AI|ClearFocus (AI|GetAIController _rook))
  (Transformation|SetActorRotation _rook (Math|Conversions|RotationFromXVector (Class|KismetMathLibrary|VectorLeft)))
  (Transformation|SetActorLocation _rook (Transformation|GetActorLocation (Variables|Default|GetTarget)) false true)
  (Variables|/Game/ThirdPerson/Blueprints/CrowCharacter_BP.CrowCharacter_BP_C|SetConversationStruct _rook_2 (Utilities|Struct|MakeConversationStruct (Utilities|Array|MakeArray "FIRST_TASK_COMPLETE" "FIRST_TASK_COMPLETE1" "FIRST_TASK_COMPLETE2" "FIRST_TASK_COMPLETE3") "Rook the Keeper"))
  (EventDispatchers|AssignConversationFinished _rook_2 (delegate Custom|BriefConversationFinished))
  (Default|EnableOuterTrigger (Variables|Default|GetGeneralScenario)))

(event Custom|BriefConversationFinished
  (bind _generalscenario (Variables|Default|GetGeneralScenario))
  (bind _generalscenario_2 (Variables|Default|GetGeneralScenario))
  (bind _rook (Variables|/Game/Blueprints/LevelScenario.LevelScenario_C|GetRook _generalscenario))
  (EventDispatchers|UnbindEventfromConversationFinished _rook (delegate Custom|BriefConversationFinished))
  (Default|MoveRooktoWaiting _generalscenario)
  (Variables|/Game/ThirdPerson/Blueprints/CrowCharacter_BP.CrowCharacter_BP_C|SetConversationStruct _rook (Utilities|Struct|MakeConversationStruct (Utilities|Array|MakeArray "Go on, find that trinket.") "Rook the Keeper"))
  (bind _asbp_third_person_character (Utilities|Casting|CastToBP_ThirdPersonCharacter (Game|Player|GetPlayerPawn 0)))
  (Default|SetMission _asbp_third_person_character "Find the widow's trinket.")
  (Default|EnableInnerTrigger _generalscenario_2)
  (Default|OpenGate _generalscenario_2)
  (Default|PlayLevelMusic _generalscenario_2)
  (Default|ActivateScenario (Variables|Default|GetLevel2)))

(event EventBeginPlay
  (EventDispatchers|AssignOnPecked (Variables|Default|GetWalnut) (delegate Custom|WalnutPecked)))

(fn ConstructionScript)