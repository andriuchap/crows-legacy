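; PeckableActor_BP is an actor that the third-person character can peck, which destroys it.
; Its Box overlap registers it as the character's current peckable and clears that on exit.
; Peck fires the OnPecked dispatcher before destroying the actor.
; SetPeckable toggles visibility and box collision profile together, and BeginPlay hides and disables the actor unless BeginPeckable is set.
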(event OnComponentBeginOverlap(Box)
  (params (OverlappedComponent :type Primitive%20Component%20Object%20Reference) (OtherActor :type Actor%20Object%20Reference) (OtherComp :type Primitive%20Component%20Object%20Reference) (OtherBodyIndex :type Integer) (bFromSweep :type Boolean) (SweepResult :type Hit%20Result%20Structure%20%28by%20ref%29))
  (bind _asbp_third_person_character (Utilities|Casting|CastToBP_ThirdPersonCharacter OtherActor))
  (Default|SetCurrentPeckable _asbp_third_person_character self))

(event OnComponentEndOverlap(Box)
  (params (OverlappedComponent :type Primitive%20Component%20Object%20Reference) (OtherActor :type Actor%20Object%20Reference) (OtherComp :type Primitive%20Component%20Object%20Reference) (OtherBodyIndex :type Integer))
  (bind _asbp_third_person_character (Utilities|Casting|CastToBP_ThirdPersonCharacter OtherActor))
  (Default|ClearPeckable _asbp_third_person_character))

(event Custom|Peck
  (Default|CallOnPecked)
  (Actor|DestroyActor))

(event Custom|SetPeckable
  (params (IsPeckable :type Boolean))
  (if IsPeckable
    (Rendering|SetVisibility (Variables|Default|GetRoot) true true)
    (Collision|SetCollisionProfileName (Variables|Default|GetBox) "OverlapOnlyPawn" true :!class /Script/Engine.PrimitiveComponent)
    (else
      (Rendering|SetVisibility (Variables|Default|GetRoot) false true)
      (Collision|SetCollisionProfileName (Variables|Default|GetBox) "NoCollision" true :!class /Script/Engine.PrimitiveComponent))))

(event EventBeginPlay
  (if (not (Variables|Default|GetBegin%20Peckable))
    (CallFunction|SetPeckable false)))

(fn ConstructionScript)