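; Level scenario actor that scripts the quest flow around Rook the Keeper, starting the walnut-retrieval mission when his first conversation finishes.
; A ScenarioProgress switch, with only the first stage implemented, sets the player's mission, plays the gate-opening sequence, walks Rook to a waiting spot, swaps his dialogue and starts music, then unbinds.
; Separate events, not called here, snap the gates open, enable inner and outer triggers, and fade music on mission completion.
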(event Custom|ConversationFinished_Event
  (switch int (Variables|Default|GetScenarioProgress)
    (:0
      (bind _asbp_third_person_character (Utilities|Casting|CastToBP_ThirdPersonCharacter (Game|Player|GetPlayerPawn 0)))
      (Default|SetMission _asbp_third_person_character "Find the walnut and return it to Rook the Keeper.")
      (Variables|Default|SetScenarioProgress (+ (Variables|Default|GetScenarioProgress) 1))
      (CallFunction|OpenGate)
      (CallFunction|MoveRooktoWaiting)
      (Variables|/Game/ThirdPerson/Blueprints/CrowCharacter_BP.CrowCharacter_BP_C|SetConversationStruct (Variables|Default|GetRook) (Utilities|Struct|MakeConversationStruct (Utilities|Array|MakeArray "FIRST_TASK_IN_PROGRESS") "Rook the Keeper"))
      (CallFunction|PlayLevelMusic)
      (EventDispatchers|UnbindEventfromConversationFinished (Variables|Default|GetRook) (delegate Custom|ConversationFinished_Event)))))

(event Custom|MissionComplete
  (CallFunction|StopLevelMusic))

(event Custom|StopLevelMusic
  (Audio|Components|Audio|FadeOut (Variables|/Script/Engine.AmbientSound|GetAudioComponent (Variables|Default|GetLevelSoundtrack)) 2.0 0.0 "Linear" :!class /Script/Engine.AudioComponent))

(event Custom|SnapGateOpen
  (Transformation|SetWorldRotation (Variables|/Script/Engine.StaticMeshActor|GetStaticMeshComponent (Variables|Default|GetLeftGate)) "0.000000,-90.000000,0.000000" false false)
  (Transformation|SetWorldRotation (Variables|/Script/Engine.StaticMeshActor|GetStaticMeshComponent (Variables|Default|GetRightGate)) "0.000000,-70.000000,0.000000" false false))

(event Custom|MoveRookToWaiting
  (AI|AIMoveTo (AI|GetAIController (Variables|Default|GetRook)) "0, 0, 0" (Variables|Default|GetWalkToTarget) 5.0 "Default" "Default" true true
    (:OnMoveFinished
      (AI|SetFocalPoint (AI|GetAIController (Variables|Default|GetRook)) (Transformation|GetActorLocation (Variables|Default|GetFaceTarget))))))

(event Custom|EnableInnerTrigger
  (Variables|/Game/Blueprints/GateCloseTrigger_BP.GateCloseTrigger_BP_C|SetEnabled (Variables|Default|GetInnerTrigger) true))

(event Custom|EnableOuterTrigger
  (Variables|/Game/Blueprints/GateCloseTrigger_BP.GateCloseTrigger_BP_C|SetEnabled (Variables|Default|GetOuterTrigger) true))

(event Custom|OpenGate
  (Sequencer|Player|Play (Variables|/Script/LevelSequence.LevelSequenceActor|GetSequencePlayer (Variables|Default|GetGateOpenSequence)) :!class /Script/MovieScene.MovieSceneSequencePlayer))

(event Custom|PlayLevelMusic
  (Audio|Components|Audio|Play (Variables|/Script/Engine.AmbientSound|GetAudioComponent (Variables|Default|GetLevelSoundtrack)) 0.0))

(event EventBeginPlay
  (EventDispatchers|AssignConversationFinished (Variables|Default|GetRook) (delegate Custom|ConversationFinished_Event)))

(fn ConstructionScript)