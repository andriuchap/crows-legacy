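; GravestoneController_BP is a level-wide manager that shows and hides the switchable gravestones to change their layout.
; On BeginPlay it gathers every SwitchableGravestone_BP actor and records the indices of those not set to start disappeared.
; Its events hide all gravestones, restore that initial layout, show only a given set, or reveal a given set additively, all through each gravestone's SetDisappeared.
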(event Custom|SetLayoutDefault
  (CallFunction|DisappearAll)
  (for _array_element (Variables|Default|GetOriginallyEnabledGravestones)
    (Default|SetDisappeared (Utilities|Array|Get(acopy) (Variables|Default|GetAllGravestones) _array_element) false)))

(event Custom|SetShowOnlySpecified
  (params (Gravestones :type Array%20of%20Switchable%20Gravestone%20BP%20Object%20References))
  (CallFunction|DisappearAll)
  (for _array_element Gravestones
    (Default|SetDisappeared _array_element false)))

(event Custom|DisappearAll
  (for _array_element (Variables|Default|GetAllGravestones)
    (Default|SetDisappeared _array_element true)))

(event Custom|SetShowSpecified
  (params (InGravestones :type Array%20of%20Switchable%20Gravestone%20BP%20Object%20References))
  (for _array_element InGravestones
    (Default|SetDisappeared _array_element false)))

(event EventBeginPlay
  (bind _outactors (Actor|GetAllActorsOfClass "/Game/Blueprints/SwitchableGravestone_BP.SwitchableGravestone_BP_C"))
  (bind _output_get (Variables|Default|SetAllGravestones _outactors))
  (for (_array_element _array_index) _output_get
    (if (not (Variables|/Game/Blueprints/SwitchableGravestone_BP.SwitchableGravestone_BP_C|GetbStartDisappeared _array_element))
      (Utilities|Array|Add (Variables|Default|GetOriginallyEnabledGravestones) _array_index))))

(fn ConstructionScript)