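; SwitchableGravestone_BP is a gravestone that switches between a present state and a disappeared state.
; On BeginPlay it caches the mesh's location, computes a drop distance from its bounds height plus a skin margin, and applies the StartDisappeared state.
; SetDisappeared instantly either hides the mesh, disables collision and moves it down by that distance, or restores visibility, collision and original location.
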(event Custom|SetDisappeared
  (params (InDisappear :type Boolean))
  (bind _staticmeshcomponent (Variables|Debug|GetStaticMeshComponent))
  (bind _staticmeshcomponent_2 (Variables|Debug|GetStaticMeshComponent))
  (if InDisappear
    (Collision|SetCollisionEnabled _staticmeshcomponent "NoCollision")
    (Rendering|SetVisibility _staticmeshcomponent false false)
    (Transformation|SetWorldLocation (Variables|Debug|GetStaticMeshComponent) (- (Variables|Default|GetStartingLocation) (Math|Vector|MakeVector 0.0 0.0 (Variables|Default|GetDisappearDistance))) false false)
    (else
      (Collision|SetCollisionEnabled _staticmeshcomponent_2 "QueryAndPhysics")
      (Rendering|SetVisibility _staticmeshcomponent_2 true false)
      (Transformation|SetWorldLocation (Variables|Debug|GetStaticMeshComponent) (Variables|Default|GetStartingLocation) false false))))

(event EventBeginPlay
  (Variables|Default|SetStartingLocation (Transformation|GetWorldLocation (Variables|Debug|GetStaticMeshComponent)))
  (Variables|Default|SetDisappearDistance (+ (* (.Z (Math|Vector|BreakVector (.BoxExtent (Collision|GetComponentBounds (Variables|Debug|GetStaticMeshComponent))))) 2.0) (Variables|Default|GetDisappearSkin)))
  (CallFunction|SetDisappeared (Variables|Default|GetbStartDisappeared)))

(fn ConstructionScript)